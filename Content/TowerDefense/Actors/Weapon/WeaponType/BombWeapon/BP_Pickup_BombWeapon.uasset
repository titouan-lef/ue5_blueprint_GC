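; Weapon pickup actor that gives the first-person character a bomb weapon in the tower defense game.
; On sphere overlap, InitWeaponComponent checks the other actor, then a bomb weapon component is added to the character and the pickup removes itself.
; The InitWeapon function repeats the same logic, with the added component class as the part that varies per weapon type.
; Construction defers to the parent class.
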(event OnComponentBeginOverlap(SphereCollision)
  (params (OverlappedComponent :type Primitive%20Component%20Object%20Reference) (OtherActor :type Actor%20Object%20Reference) (OtherComp :type Primitive%20Component%20Object%20Reference) (OtherBodyIndex :type Integer) (bFromSweep :type Boolean) (SweepResult :type Hit%20Result%20Structure%20%28by%20ref%29))
  (bind _sucess (CallFunction|InitWeaponComponent OtherActor))
  (if _sucess
    ;[1 1 1] BP to change depending on the class
    (AddComponent|AddBPBombWeaponComponent (Variables|Default|GetFirstPersonCharacterReference) false)
    (CallFunction|RemovePickUp)))

(event EventBeginPlay)

(event Collision|EventActorBeginOverlap
  (params (OtherActor :type Actor%20Object%20Reference)))

(event EventTick
  (params (DeltaSeconds :type Float%20%28single-precision%29)))

(fn ConstructionScript
  (|CallParentFunction))

(fn InitWeapon
  (params (Other%20Actor :type Actor%20Object%20Reference))
  (bind _sucess (CallFunction|InitWeaponComponent Other%20Actor))
  (if _sucess
    ;[1 1 1] BP to change depending on the class
    (AddComponent|AddBPBombWeaponComponent (Variables|Default|GetFirstPersonCharacterReference) false)
    (CallFunction|RemovePickUp)))