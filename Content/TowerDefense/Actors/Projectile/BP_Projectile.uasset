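; BP_Projectile is a projectile actor for the tower defense game, moved by a ProjectileMovement component.
; The construction script copies its Speed variable into the movement component's initial speed.
; On BeginPlay a one-shot timer destroys the actor after a fixed lifetime.
; An InvisibleBullet function hides the Bullet component and its children, though nothing in this Blueprint calls it.
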(event Custom|DeathByTime
  (Actor|DestroyActor))

(event EventBeginPlay
  (Utilities|Time|SetTimerbyEvent (delegate Custom|DeathByTime) 1e+01))

(fn ConstructionScript
  (CallFunction|SetSpeed))

(fn SetSpeed
  (Variables|/Script/Engine.ProjectileMovementComponent|SetInitialSpeed (Variables|Default|GetProjectileMovement) (Variables|Default|Getspeed))
  (return))

(fn InvisibleBullet
  (Rendering|SetVisibility (Variables|Default|GetBullet) false true))