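; BP_Tower is a destructible tower pawn in the tower defense game that takes damage from enemy hitboxes.
; Box overlaps with BP_HitBoxEnemy pass the hitbox's damage to ACLifeSystem and briefly flash two point lights to the damage color.
; Tick copies health to a life bar widget rotated toward the player, and polls for death.
; Death hides the monument mesh, activates a Niagara effect, then destroys the actor after a delay.
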(event OnComponentBeginOverlap(Box)
  (params (OverlappedComponent :type Primitive%20Component%20Object%20Reference) (OtherActor :type Actor%20Object%20Reference) (OtherComp :type Primitive%20Component%20Object%20Reference) (OtherBodyIndex :type Integer) (bFromSweep :type Boolean) (SweepResult :type Hit%20Result%20Structure%20%28by%20ref%29))
  (if (== (Utilities|GetClass OtherActor) "/Game/TowerDefense/Actors/HitBox/BP_HitBoxEnemy.BP_HitBoxEnemy_C")
    (bind _asbp_hit_box (Utilities|Casting|CastToBP_HitBox OtherActor)
      (:then
        (Default|TakeDamage (Variables|Default|GetAC_LifeSystem) (Variables|/Game/TowerDefense/Actors/HitBox/BP_HitBox.BP_HitBox_C|GetDamage _asbp_hit_box))
        (CallFunction|ChangeLightColor (Variables|Default|GetColorDamage))
        (Utilities|FlowControl|Delay 0.5)
        (CallFunction|ChangeLightColor (Variables|Default|GetColorGood))
        (Development|PrintString (Utilities|String|ToString(Float) (Variables|/Game/TowerDefense/Actors/HitBox/BP_HitBox.BP_HitBox_C|GetDamage _asbp_hit_box))))
      (:CastFailed
        (Development|PrintString "Can't cast Hitbox !")))))

(event Custom|Death
  (Rendering|SetVisibility (Variables|Default|GetSM_Monument_06) false true)
  (Components|Activation|Activate (Variables|Default|GetNiagara) true)
  (Utilities|FlowControl|Delay 1.0)
  (Actor|DestroyActor))

(event EventTick
  (params (DeltaSeconds :type Float%20%28single-precision%29))
  (CallFunction|UpdateLB)
  (if (Default|IsDead? (Variables|Default|GetAC_LifeSystem))
    (CallFunction|Death)))

(fn ConstructionScript)

(fn ChangeLightColor
  (params (Color :type Linear%20Color%20Structure))
  (Rendering|Components|Light|SetLightColor (Variables|Default|GetPointLight) Color true)
  (Rendering|Components|Light|SetLightColor (Variables|Default|GetPointLight1) Color true))

(fn UpdateLB
  (bind _aswp_ialife_bar (Utilities|Casting|CastToWP_IALifeBar (UserInterface|GetUserWidgetObject (Variables|Default|GetLB))))
  (Variables|/Game/TowerDefense/Actors/Pawn/Enemy/Zombie/WP_IALifeBar.WP_IALifeBar_C|SetHealth _aswp_ialife_bar (Variables|/Game/AC_LifeSystem.AC_LifeSystem_C|GetCurrentHealth (Variables|Default|GetAC_LifeSystem)))
  (Transformation|SetWorldRotation (Variables|Default|GetLB) (Math|Rotator|FindLookatRotation (Transformation|GetActorLocation self) (Transformation|GetActorLocation (Game|Player|GetPlayerPawn 0))) false false)
  (return))