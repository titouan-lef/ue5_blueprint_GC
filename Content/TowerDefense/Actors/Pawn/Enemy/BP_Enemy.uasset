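; BP_Enemy is the enemy pawn for the tower defense game, tracking health through its LifeSystem.
; The AffectHealth event ignores enemies that are already dead, otherwise adds a signed delta to current health and recomputes the dead flag at zero or below.
; On death it detaches from its controller pending destroy; the pawn itself is not destroyed in these graphs.
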(event EventBeginPlay)

(event Collision|EventActorBeginOverlap
  (params (OtherActor :type Actor%20Object%20Reference)))

(event EventTick
  (params (DeltaSeconds :type Float%20%28single-precision%29)))

(event EventAffectHealth
  (params (delta :type Float%20%28double-precision%29))
  (if (not (Variables|/Game/TowerDefense/Actors/AC_LifeSystem.AC_LifeSystem_C|GetIsDead (Variables|Default|GetLifeSystem)))
    (CallFunction|UpdateHealthPoints delta)
    (if (Variables|/Game/TowerDefense/Actors/AC_LifeSystem.AC_LifeSystem_C|GetIsDead (Variables|Default|GetLifeSystem))
      (Class|Pawn|DetachfromControllerPendingDestroy))))

(fn ConstructionScript)

(fn UpdateHealthPoints
  (params (delta :type Float%20%28double-precision%29))
  (bind _lifesystem (Variables|Default|GetLifeSystem))
  (bind _output_get (Variables|/Game/TowerDefense/Actors/AC_LifeSystem.AC_LifeSystem_C|SetCurrentHealth _lifesystem (+ delta (Variables|/Game/TowerDefense/Actors/AC_LifeSystem.AC_LifeSystem_C|GetCurrentHealth _lifesystem))))
  (CallFunction|UpdateIsDead)
  (return _output_get))

(fn UpdateIsDead
  (bind _lifesystem (Variables|Default|GetLifeSystem))
  (Variables|/Game/TowerDefense/Actors/AC_LifeSystem.AC_LifeSystem_C|SetIsDead _lifesystem (<= (Variables|/Game/TowerDefense/Actors/AC_LifeSystem.AC_LifeSystem_C|GetCurrentHealth _lifesystem) 0.0))
  (return))