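; Zombie enemy for the tower defense game that chases the player pawn and melee-attacks it.
; Tick reissues AI MoveTo; successful moves accumulate a timer that periodically raises Attacking and briefly enables overlap events on the BPHitBoxEnemy child sphere.
; A widget life bar takes max health from LifeSystem at start, then updates current health and rotates toward the player every tick.
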(event EventBeginPlay
  (bind _aswp_ialife_bar (Utilities|Casting|CastToWP_IALifeBar (UserInterface|GetUserWidgetObject (Variables|Default|GetWidget))))
  (Default|SetHealth _aswp_ialife_bar (Variables|/Game/AC_LifeSystem.AC_LifeSystem_C|GetMaxHealth (Variables|Default|GetLifeSystem)))
  (bind _assphere_collision (CallFunction|GetSphere))
  (Variables|/Script/Engine.PrimitiveComponent|SetbGenerateOverlapEvents _assphere_collision false))

(event EventTick
  (params (DeltaSeconds :type Float%20%28single-precision%29))
  (CallFunction|UpdateLifeBar)
  (AI|AIMoveTo self "0, 0, 0" (Game|Player|GetPlayerPawn 0) 6e+01 false
    (:OnSuccess
      (bind _output_get (Variables|Default|SetTime (+ DeltaSeconds (Variables|Default|GetTime))))
      (Math|Float|CompareFloat _output_get 2.0
        (:>
          (Variables|Default|SetTime 0.0)
          (Variables|Default|SetAttacking true)
          (bind _assphere_collision (CallFunction|GetSphere))
          (Variables|/Script/Engine.PrimitiveComponent|SetbGenerateOverlapEvents _assphere_collision true)
          (Utilities|FlowControl|Delay 1.1)
          (bind _assphere_collision_2 (CallFunction|GetSphere))
          (Variables|/Script/Engine.PrimitiveComponent|SetbGenerateOverlapEvents _assphere_collision_2 false)
          (Variables|Default|SetAttacking false))))))

(fn ConstructionScript
  (|CallParentFunction))

(fn UpdateLifeBar
  (bind _widget (Variables|Default|GetWidget))
  (bind _aswp_ialife_bar (Utilities|Casting|CastToWP_IALifeBar (UserInterface|GetUserWidgetObject _widget)))
  (Variables|/Game/TowerDefense/Actors/Pawn/Enemy/Zombie/WP_IALifeBar.WP_IALifeBar_C|SetHealth _aswp_ialife_bar (Variables|/Game/AC_LifeSystem.AC_LifeSystem_C|GetCurrentHealth (Variables|Default|GetLifeSystem)))
  (Transformation|SetWorldRotation _widget (Math|Rotator|FindLookatRotation (Transformation|GetActorLocation self) (Transformation|GetActorLocation (Game|Player|GetPlayerPawn 0))) false false))

(fn GetSphere
  (bind _assphere_collision (Utilities|Casting|CastToSphereComponent (Components|GetChildComponent (Components|GetChildComponent (Variables|Default|GetBP_HitBoxEnemy) 0) 0)))
  (return _assphere_collision))