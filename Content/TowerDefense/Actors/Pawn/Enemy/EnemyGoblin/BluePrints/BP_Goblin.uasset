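; Goblin enemy pawn for the tower defense game that seeks out and attacks towers.
; While alive, Tick targets the BP_Tower with the lowest Priority value and issues AIMoveTo.
; Successful moves accumulate time toward periodic attacks, which briefly enable overlaps on the child hitbox sphere.
; Player hitbox overlaps damage LifeSystem and update the life bar, turning it toward the player; death detaches the controller and destroys the goblin after a delay.
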(event OnComponentBeginOverlap(CapsuleComponent)
  (params (OverlappedComponent :type Primitive%20Component%20Object%20Reference) (OtherActor :type Actor%20Object%20Reference) (OtherComp :type Primitive%20Component%20Object%20Reference) (OtherBodyIndex :type Integer) (bFromSweep :type Boolean) (SweepResult :type Hit%20Result%20Structure%20%28by%20ref%29))
  (bind _lifesystem (Variables|Default|GetLifeSystem))
  ;[1 1 1] Damaged
  (if (== (Utilities|GetClass OtherActor) "/Game/TowerDefense/Actors/HitBox/BP_HitBoxPlayer.BP_HitBoxPlayer_C")
    (bind _asbp_hit_box (Utilities|Casting|CastToBP_HitBox OtherActor))
    (Default|TakeDamage _lifesystem (Variables|/Game/TowerDefense/Actors/HitBox/BP_HitBox.BP_HitBox_C|GetDamage _asbp_hit_box))
    (CallFunction|UpdateLife)
    (if (Default|IsDead? _lifesystem)
      (Class|Pawn|DetachfromControllerPendingDestroy)
      (Utilities|FlowControl|Delay 1.0)
      (Actor|DestroyActor))))

(event Custom|CustomEvent
  ;[1 1 1] Move And Attack
  (bind _assphere_collision (CallFunction|GetSphere))
  (Variables|/Script/Engine.PrimitiveComponent|SetbGenerateOverlapEvents _assphere_collision false)
  (Variables|Default|SetAttacking false))

(event EventBeginPlay
  ;[1 1 1] Deactivate Initial Hitbox
  (bind _assphere_collision (CallFunction|GetSphere))
  (Variables|/Script/Engine.PrimitiveComponent|SetbGenerateOverlapEvents _assphere_collision false)
  ;[1 1 1] Life Bar
  (bind _aswp_ialife_bar (Utilities|Casting|CastToWP_IALifeBar (UserInterface|GetUserWidgetObject (Variables|Default|GetLB))))
  (Default|SetHealth _aswp_ialife_bar (Variables|/Game/AC_LifeSystem.AC_LifeSystem_C|GetMaxHealth (Variables|Default|GetLifeSystem))))

(event EventTick
  (params (DeltaSeconds :type Float%20%28single-precision%29))
  ;[1 1 1] Move And Attack
  (if (not (Default|IsDead? (Variables|Default|GetLifeSystem)))
    (CallFunction|SetTarget)
    (AI|AIMoveTo (Class|PawnMovementComponent|GetPawnOwner (Variables|Character|GetCharacterMovement)) "0, 0, 0" (Variables|Default|GetTarget) 5e+02 false
      (:OnSuccess
        (bind _output_get (Variables|Default|SetTime (+ DeltaSeconds (Variables|Default|GetTime))))
        (Math|Float|CompareFloat _output_get 2.0
          (:>
            (Variables|Default|SetTime 0.0)
            (Variables|Default|SetAttacking true)
            (bind _assphere_collision (CallFunction|GetSphere))
            (Variables|/Script/Engine.PrimitiveComponent|SetbGenerateOverlapEvents _assphere_collision true)
            (Utilities|Time|SetTimerbyEvent (delegate Custom|CustomEvent) 1.1)))))))

(fn ConstructionScript)

(fn UpdateLife
  (bind _lifesystem (Variables|Default|GetLifeSystem))
  (bind _aswp_ialife_bar (Utilities|Casting|CastToWP_IALifeBar (UserInterface|GetUserWidgetObject (Variables|Default|GetLB))))
  (Variables|/Game/TowerDefense/Actors/Pawn/Enemy/Zombie/WP_IALifeBar.WP_IALifeBar_C|SetHealth _aswp_ialife_bar (* (/ (Variables|/Game/AC_LifeSystem.AC_LifeSystem_C|GetCurrentHealth _lifesystem) (Variables|/Game/AC_LifeSystem.AC_LifeSystem_C|GetMaxHealth _lifesystem)) 1e+02))
  (Transformation|SetWorldRotation (Variables|Default|GetLB) (Math|Rotator|FindLookatRotation (Transformation|GetActorLocation self) (Transformation|GetActorLocation (Game|Player|GetPlayerPawn 0))) false false)
  (return))

(fn SetTarget
  (bind _outactors (Actor|GetAllActorsOfClass "/Game/TowerDefense/Actors/Pawn/BP_Tower.BP_Tower_C"))
  (bind _output_get (LocalVariables|SetTowerArray _outactors))
  (for (_ _array_index) _output_get
    (if (== (Variables|/Game/TowerDefense/Actors/Pawn/BP_Tower.BP_Tower_C|GetPriority (Utilities|Array|Get(acopy) (LocalVariables|GetTowerArray) _array_index)) 0)
      (bind _output_get_2 (LocalVariables|SetTempTarget (Utilities|Array|Get(acopy) (LocalVariables|GetTowerArray) _array_index)))
      (Variables|Default|Settarget _output_get_2)
      (return)
      (else
        (Utilities|IsValid (LocalVariables|GetTempTarget)
          (:Is%20Valid
            (if (not (< (Variables|/Game/TowerDefense/Actors/Pawn/BP_Tower.BP_Tower_C|GetPriority (LocalVariables|GetTempTarget)) (Variables|/Game/TowerDefense/Actors/Pawn/BP_Tower.BP_Tower_C|GetPriority (Utilities|Array|Get(acopy) (LocalVariables|GetTowerArray) _array_index))))
              (LocalVariables|SetTempTarget (Utilities|Array|Get(acopy) (LocalVariables|GetTowerArray) _array_index))))
          (:Is%20Not%20Valid
            (LocalVariables|SetTempTarget (Utilities|Array|Get(acopy) (LocalVariables|GetTowerArray) _array_index)))))))
  (Variables|Default|SetTarget (LocalVariables|GetTempTarget))
  (return))

(fn GetSphere
  (bind _assphere_collision (Utilities|Casting|CastToSphereComponent (Components|GetChildComponent (Components|GetChildComponent (Variables|Default|GetBP_HitBoxEnemy) 0) 0)))
  (return _assphere_collision))