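; BP_Skeleton is a tower defense enemy that raids towers with arrows.
; On a looping timer it targets the tower with the lowest Priority value, moves within range via AIMoveTo, faces it and launches an impulse-driven BP_Arrows.
; Player hitbox overlaps damage its LifeSystem, triggering a brief hit state or a Niagara death effect before destruction.
; Tick updates the health bar widget and turns it toward the player.
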(event OnComponentBeginOverlap(CapsuleComponent)
  (params (OverlappedComponent :type Primitive%20Component%20Object%20Reference) (OtherActor :type Actor%20Object%20Reference) (OtherComp :type Primitive%20Component%20Object%20Reference) (OtherBodyIndex :type Integer) (bFromSweep :type Boolean) (SweepResult :type Hit%20Result%20Structure%20%28by%20ref%29))
  (bind _lifesystem (Variables|Default|GetLifeSystem))
  (if (== (Utilities|GetClass OtherActor) "/Game/TowerDefense/Actors/HitBox/BP_HitBoxPlayer.BP_HitBoxPlayer_C")
    (bind _asbp_hit_box (Utilities|Casting|CastToBP_HitBox OtherActor)
      (:then
        (Default|TakeDamage _lifesystem (Variables|/Game/TowerDefense/Actors/HitBox/BP_HitBox.BP_HitBox_C|GetDamage _asbp_hit_box))
        (if (Default|IsDead? _lifesystem)
          (Rendering|SetVisibility (Variables|Default|GetNiagaraDeath) true false)
          (Utilities|FlowControl|Delay 1.0)
          (Actor|DestroyActor)
          (else
            (Variables|Default|SetIsHit true)
            (Utilities|FlowControl|Delay 0.5)
            (Variables|Default|SetIsHit false))))
      (:CastFailed
        (Development|PrintString "Something gone wrong..." true true "(R=1.000000,G=0.000000,B=0.024324,A=1.000000)")))))

(event Custom|RaidTower
  (bind _target (Variables|Default|Gettarget))
  (bind _charactermovement (Variables|Character|GetCharacterMovement))
  (bind _returnvalue (Class|PawnMovementComponent|GetPawnOwner _charactermovement))
  (CallFunction|SetTarget)
  (AI|AIMoveTo _returnvalue "0, 0, 0" _target 2e+03 true
    (:OnSuccess
      (Transformation|SetActorRotation (Class|PawnMovementComponent|GetPawnOwner (Variables|Character|GetCharacterMovement)) (Math|Rotator|FindLookatRotation (Transformation|GetActorLocation _returnvalue) (Transformation|GetActorLocation _target)) true)
      (CallFunction|AttackTower))))

(event Custom|AttackTower
  (Variables|Default|SetisInRange true)
  (Utilities|FlowControl|Delay 0.5)
  (CallFunction|Attack))

(event EventBeginPlay
  (bind _aswp_ialife_bar (Utilities|Casting|CastToWP_IALifeBar (UserInterface|GetUserWidgetObject (Variables|Default|GetLifeBar))))
  (Default|SetHealth _aswp_ialife_bar (Variables|/Game/TowerDefense/Actors/AC_LifeSystem.AC_LifeSystem_C|GetMaxHealth (Variables|Default|GetLifeSystem)))
  (Utilities|Time|SetTimerbyEvent (delegate Custom|RaidTower) (Variables|Default|GetShotSpeed) true))

(event EventTick
  (params (DeltaSeconds :type Float%20%28single-precision%29))
  (CallFunction|UpdateLifeBar))

(fn ConstructionScript
  (|CallParentFunction))

(fn SetTarget
  (bind _outactors (Actor|GetAllActorsOfClass "/Game/TowerDefense/Actors/Pawn/BP_Tower.BP_Tower_C"))
  (bind _output_get (LocalVariables|SetTowerArray _outactors))
  (for (_ _array_index) _output_get
    (if (== (Variables|/Game/TowerDefense/Actors/Pawn/BP_Tower.BP_Tower_C|GetPriority (Utilities|Array|Get(acopy) (LocalVariables|GetTowerArray) _array_index)) 0)
      (bind _output_get_2 (LocalVariables|SetTempTarget (Utilities|Array|Get(acopy) (LocalVariables|GetTowerArray) _array_index)))
      (Variables|Default|Settarget _output_get_2)
      (return)
      (else
        (Utilities|IsValid (LocalVariables|GetTempTarget)
          (:Is%20Valid
            (if (not (< (Variables|/Game/TowerDefense/Actors/Pawn/BP_Tower.BP_Tower_C|GetPriority (LocalVariables|GetTempTarget)) (Variables|/Game/TowerDefense/Actors/Pawn/BP_Tower.BP_Tower_C|GetPriority (Utilities|Array|Get(acopy) (LocalVariables|GetTowerArray) _array_index))))
              (LocalVariables|SetTempTarget (Utilities|Array|Get(acopy) (LocalVariables|GetTowerArray) _array_index))))
          (:Is%20Not%20Valid
            (LocalVariables|SetTempTarget (Utilities|Array|Get(acopy) (LocalVariables|GetTowerArray) _array_index)))))))
  (Variables|Default|Settarget (LocalVariables|GetTempTarget))
  (return))

(fn Attack
  (bind _returnvalue (Game|SpawnActorfromClass "/Game/TowerDefense/Actors/Projectile/BP_Arrows.BP_Arrows_C" (Math|Transform|MakeTransform (+ (+ (Transformation|GetActorLocation) (* (Transformation|GetActorForwardVector) "100.000000,100.000000,100.000000")) "0.000000,0.000000,50.000000") (Transformation|GetActorRotation) "10.000000,10.000000,10.000000") "Undefined" "MultiplyWithRoot" 0 0))
  (Physics|AddImpulse (Variables|/Game/TowerDefense/Actors/Projectile/BP_Arrows.BP_Arrows_C|GetSphereCollision _returnvalue) (* (Transformation|GetActorForwardVector) (Variables|Default|GetForce)) "None" false)
  (Variables|Default|SetisInRange false))

(fn UpdateLifeBar
  (bind _lifebar (Variables|Default|GetLifeBar))
  (bind _aswp_ialife_bar (Utilities|Casting|CastToWP_IALifeBar (UserInterface|GetUserWidgetObject _lifebar)))
  (Variables|/Game/TowerDefense/Actors/Pawn/Enemy/Zombie/WP_IALifeBar.WP_IALifeBar_C|SetHealth _aswp_ialife_bar (Variables|/Game/TowerDefense/Actors/AC_LifeSystem.AC_LifeSystem_C|GetCurrentHealth (Variables|Default|GetLifeSystem)))
  (Transformation|SetWorldRotation _lifebar (Math|Rotator|FindLookatRotation (Transformation|GetActorLocation self) (Transformation|GetActorLocation (Game|Player|GetPlayerPawn 0))) false false))