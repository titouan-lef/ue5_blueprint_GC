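; BP_OrbLich is the Lich enemy's energy orb actor, which explodes when its sphere hits something.
; The hit calls OnDestroy, which removes the sphere, enemy hitbox and energy ball effect, activates the explosion effect, then destroys the actor after a short delay.
; An impulse that would push the player away is unconnected, so the explosion overlap does nothing; a note says it needs physics simulation on the player capsule.
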(event OnComponentHit(Sphere)
  (params (HitComponent :type Primitive%20Component%20Object%20Reference) (OtherActor :type Actor%20Object%20Reference) (OtherComp :type Primitive%20Component%20Object%20Reference) (NormalImpulse :type Vector :default "0, 0, 0") (Hit :type Hit%20Result%20Structure%20%28by%20ref%29))
  (CallFunction|OnDestroy))

(event OnComponentBeginOverlap(SphereExplosion)
  (params (OverlappedComponent :type Primitive%20Component%20Object%20Reference) (OtherActor :type Actor%20Object%20Reference) (OtherComp :type Primitive%20Component%20Object%20Reference) (OtherBodyIndex :type Integer) (bFromSweep :type Boolean) (SweepResult :type Hit%20Result%20Structure%20%28by%20ref%29))
  ;[1 1 1] Need To Simulate Physics on Player capsule
)

(event Custom|OnDestroy
  (Components|DestroyComponent (Variables|Default|GetSphere))
  (Components|DestroyComponent (Variables|Default|GetBP_HitBoxEnemy))
  (Components|DestroyComponent (Variables|Default|GetP_EnergyBall))
  (Components|Activation|Activate (Variables|Default|GetP_ExplosionEnergy_03) false)
  (Utilities|FlowControl|Delay 1.0)
  (Actor|DestroyActor))

(event EventBeginPlay)

(fn ConstructionScript)