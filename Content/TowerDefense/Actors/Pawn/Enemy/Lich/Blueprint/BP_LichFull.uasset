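; Lich enemy for the tower defense game that can fire orb projectiles and summon random minions around itself.
; A looping timer periodically halts movement and raises IsRez, while Attack does the same with IsAttacking.
; Player hitbox overlaps damage its LifeSystem, set IsHit and stop movement on death.
; SpawnOrb, LaunchOrb, CallSomeone and Death are separate steps with no callers here, leaving their timing to outside logic.
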(event OnComponentBeginOverlap(CapsuleComponent)
  (params (OverlappedComponent :type Primitive%20Component%20Object%20Reference) (OtherActor :type Actor%20Object%20Reference) (OtherComp :type Primitive%20Component%20Object%20Reference) (OtherBodyIndex :type Integer) (bFromSweep :type Boolean) (SweepResult :type Hit%20Result%20Structure%20%28by%20ref%29))
  (bind _lifesystem (Variables|Default|GetLifeSystem))
  (if (== (Utilities|GetClass OtherActor) "/Game/TowerDefense/Actors/HitBox/BP_HitBoxPlayer.BP_HitBoxPlayer_C")
    (bind _asbp_hit_box (Utilities|Casting|CastToBP_HitBox OtherActor)
      (:then
        (Default|TakeDamage _lifesystem (Variables|/Game/TowerDefense/Actors/HitBox/BP_HitBox.BP_HitBox_C|GetDamage _asbp_hit_box))
        (Variables|Default|SetIsHit true)
        (if (Default|IsDead? _lifesystem)
          (Pawn|Components|CharacterMovement|SetMovementMode (Variables|Character|GetCharacterMovement) "MOVE_None" 0)))
      (:CastFailed
        (Development|PrintString "Can't cast Hitbox !" true true "(R=1.000000,G=0.000000,B=0.024324,A=1.000000)")))))

(event Custom|Death
  (Actor|DestroyActor))

(event Custom|Calling
  (Pawn|Components|CharacterMovement|SetMovementMode (Variables|Character|GetCharacterMovement) "MOVE_None" 0)
  (Variables|Default|SetIsRez true))

(event EventBeginPlay
  (|CallParentFunction)
  (Utilities|Time|SetTimerbyEvent (delegate Custom|Calling) 2e+01 true))

(event EventTick
  (params (DeltaSeconds :type Float%20%28single-precision%29))
  (|CallParentFunction DeltaSeconds))

(fn ConstructionScript)

(fn SpawnOrb
  (bind _returnvalue (Game|SpawnActorfromClass (Variables|Default|GetProjectile) (Math|Transform|MakeTransform (+ (Transformation|GetActorLocation) (* (Transformation|GetActorForwardVector) "100.000000,100.000000,100.000000")) (Transformation|GetActorRotation)) "Undefined" "MultiplyWithRoot" 0 0))
  (Variables|Default|SetProjectileToLaunch _returnvalue))

(fn LaunchOrb
  (Physics|AddImpulse (Variables|/Game/TowerDefense/Actors/Pawn/Enemy/Lich/Blueprint/BP_OrbLich.BP_OrbLich_C|GetSphere (Variables|Default|GetProjectileToLaunch)) (* (Transformation|GetActorForwardVector) (LocalVariables|GetImpulseStrenght)) "None" false))

(fn CallSomeone
  (bind _returnvalue (Transformation|GetActorTransform))
  (bind (_location _rotation _scale) (Math|Transform|BreakTransform _returnvalue))
  (Game|SpawnActorfromClass (.OutItem (Utilities|Array|Random (Variables|Default|GetInvocs))) (Math|Transform|MakeTransform (CallFunction|GetRandomPlaceAround -5e+02 5e+02) _rotation _scale) "Undefined" "MultiplyWithRoot" 0 0))

(fn GetRandomPlaceAround
  (params (Min :type Float%20%28double-precision%29) (Max :type Float%20%28double-precision%29))
  (bind _returnvalue (Math|Random|RandomUnitVector))
  (bind (_x _y) (Math|Vector|BreakVector _returnvalue))
  (return (+ (Transformation|GetActorLocation) (* (Math|Vector|MakeVector _x _y 0.0) (Math|Random|RandomFloatinRange Min Max)))))

(fn Attack
  (Pawn|Components|CharacterMovement|SetMovementMode (Variables|Character|GetCharacterMovement) "MOVE_None" 0)
  (Variables|Default|SetIsAttacking true))