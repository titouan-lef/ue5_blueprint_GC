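; BP_VR_SpawnSphereHit is a spawner that endlessly fires BP_VR_Electric_Proj actors from its own location and rotation.
; BeginPlay waits a random delay of up to one second, then spawns projectiles in a chain separated by fixed delays.
; After each group of three and a further delay, the custom event Again jumps back to the start of the chain, looping without a timer.
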(event Custom|Again
  (Utilities|FlowControl|Delay 2.0)
  (Game|SpawnActorfromClass "/Game/TowerDefense/Stylized_VFX_StPack/VR/VR_Blueprints/BP_VR_Electric_Proj.BP_VR_Electric_Proj_C" (Math|Transform|MakeTransform (Transformation|GetActorLocation) (Transformation|GetActorRotation) "1.000000,1.000000,1.000000") "Undefined" "OverrideRootScale" 0 "(R=0.000000,G=0.651406,B=0.947307,A=1.000000)" 1.0 false 1e+03 1 0)
  (Utilities|FlowControl|Delay 2.0)
  (Game|SpawnActorfromClass "/Game/TowerDefense/Stylized_VFX_StPack/VR/VR_Blueprints/BP_VR_Electric_Proj.BP_VR_Electric_Proj_C" (Math|Transform|MakeTransform (Transformation|GetActorLocation) (Transformation|GetActorRotation) "1.000000,1.000000,1.000000") "Undefined" "OverrideRootScale" 0 "(R=0.000000,G=0.651406,B=0.947307,A=1.000000)" 1.0 false 1e+03 1 0)
  (Utilities|FlowControl|Delay 2.0)
  (Game|SpawnActorfromClass "/Game/TowerDefense/Stylized_VFX_StPack/VR/VR_Blueprints/BP_VR_Electric_Proj.BP_VR_Electric_Proj_C" (Math|Transform|MakeTransform (Transformation|GetActorLocation) (Transformation|GetActorRotation) "1.000000,1.000000,1.000000") "Undefined" "OverrideRootScale" 0 "(R=0.000000,G=0.651406,B=0.947307,A=1.000000)" 1.0 false 1e+03 1 0)
  (Utilities|FlowControl|Delay 2.0)
  (CallFunction|Again))

(event EventBeginPlay
  (Utilities|FlowControl|Delay (Math|Random|RandomFloatinRange 0.0 1.0))
  (Utilities|FlowControl|Delay 2.0)
  (Game|SpawnActorfromClass "/Game/TowerDefense/Stylized_VFX_StPack/VR/VR_Blueprints/BP_VR_Electric_Proj.BP_VR_Electric_Proj_C" (Math|Transform|MakeTransform (Transformation|GetActorLocation) (Transformation|GetActorRotation) "1.000000,1.000000,1.000000") "Undefined" "OverrideRootScale" 0 "(R=0.000000,G=0.651406,B=0.947307,A=1.000000)" 1.0 false 1e+03 1 0)
  (Utilities|FlowControl|Delay 2.0)
  (Game|SpawnActorfromClass "/Game/TowerDefense/Stylized_VFX_StPack/VR/VR_Blueprints/BP_VR_Electric_Proj.BP_VR_Electric_Proj_C" (Math|Transform|MakeTransform (Transformation|GetActorLocation) (Transformation|GetActorRotation) "1.000000,1.000000,1.000000") "Undefined" "OverrideRootScale" 0 "(R=0.000000,G=0.651406,B=0.947307,A=1.000000)" 1.0 false 1e+03 1 0)
  (Utilities|FlowControl|Delay 2.0)
  (Game|SpawnActorfromClass "/Game/TowerDefense/Stylized_VFX_StPack/VR/VR_Blueprints/BP_VR_Electric_Proj.BP_VR_Electric_Proj_C" (Math|Transform|MakeTransform (Transformation|GetActorLocation) (Transformation|GetActorRotation) "1.000000,1.000000,1.000000") "Undefined" "OverrideRootScale" 0 "(R=0.000000,G=0.651406,B=0.947307,A=1.000000)" 1.0 false 1e+03 1 0)
  (Utilities|FlowControl|Delay 2.0)
  (CallFunction|Again))

(fn ConstructionScript)