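; BP_SpawnElectric_Projectile is a spawner actor that repeatedly fires BP_Electric_Projectile from its own location and rotation.
; On BeginPlay it waits a delay scaled by Level, then spawns a projectile, passing along Gravity, ImpulsePower and Level.
; A custom Again event calls itself after each spawn, looping the fire on a fixed delay.
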(event Custom|Again
  (Utilities|FlowControl|Delay 3.0)
  (Game|SpawnActorfromClass "/Game/TowerDefense/Stylized_VFX_StPack/Blueprints/BP_Electric_Projectile.BP_Electric_Projectile_C" (Math|Transform|MakeTransform (Transformation|GetActorLocation) (Transformation|GetActorRotation) "1.000000,1.000000,1.000000") "Undefined" "OverrideRootScale" 0 "(R=0.000000,G=0.651406,B=0.947307,A=1.000000)" 1.0 (Variables|Default|GetGravity) (Variables|Default|GetImpulsePower) (Variables|Default|GetLevel) 0)
  (CallFunction|Again))

(event EventBeginPlay
  (Utilities|FlowControl|Delay (* (Variables|Default|GetLevel) 1.0))
  (Game|SpawnActorfromClass "/Game/TowerDefense/Stylized_VFX_StPack/Blueprints/BP_Electric_Projectile.BP_Electric_Projectile_C" (Math|Transform|MakeTransform (Transformation|GetActorLocation) (Transformation|GetActorRotation) "1.000000,1.000000,1.000000") "Undefined" "OverrideRootScale" 0 "(R=0.000000,G=0.651406,B=0.947307,A=1.000000)" 1.0 (Variables|Default|GetGravity) (Variables|Default|GetImpulsePower) (Variables|Default|GetLevel) 0)
  (CallFunction|Again))

(fn ConstructionScript)