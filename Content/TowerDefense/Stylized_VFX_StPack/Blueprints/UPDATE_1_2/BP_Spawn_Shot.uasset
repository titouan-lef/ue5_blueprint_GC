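; Actor from a stylized VFX pack that repeatedly plays a classic shot effect at its own location and rotation.
; Its Level value sets the initial delay in seconds on BeginPlay and selects one of three shot particle systems to spawn.
; After each spawn, the Again event calls itself through a fixed delay, creating an endless timed loop.
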(event Custom|Again
  (bind _returnvalue (Transformation|GetActorRotation))
  (bind _returnvalue_2 (Transformation|GetActorLocation))
  (Utilities|FlowControl|Delay 3.0)
  (switch int (Variables|Default|GetLevel)
    (:1
      (Niagara|SpawnSystematLocation "/Game/TowerDefense/Stylized_VFX_StPack/Particles/UPDATE_1_2/P_Classic_Shot_01.P_Classic_Shot_01" _returnvalue_2 _returnvalue))
    (:2
      (Niagara|SpawnSystematLocation "/Game/TowerDefense/Stylized_VFX_StPack/Particles/UPDATE_1_2/P_Classic_Shot_02.P_Classic_Shot_02" _returnvalue_2 _returnvalue))
    (:3
      (Niagara|SpawnSystematLocation "/Game/TowerDefense/Stylized_VFX_StPack/Particles/UPDATE_1_2/P_Classic_Shot_03.P_Classic_Shot_03" _returnvalue_2 _returnvalue)))
  (CallFunction|Again))

(event EventBeginPlay
  (bind _returnvalue (Transformation|GetActorRotation))
  (bind _returnvalue_2 (Transformation|GetActorLocation))
  (Utilities|FlowControl|Delay (* (Variables|Default|GetLevel) 1.0))
  (switch int (Variables|Default|GetLevel)
    (:1
      (Niagara|SpawnSystematLocation "/Game/TowerDefense/Stylized_VFX_StPack/Particles/UPDATE_1_2/P_Classic_Shot_01.P_Classic_Shot_01" _returnvalue_2 _returnvalue))
    (:2
      (Niagara|SpawnSystematLocation "/Game/TowerDefense/Stylized_VFX_StPack/Particles/UPDATE_1_2/P_Classic_Shot_02.P_Classic_Shot_02" _returnvalue_2 _returnvalue))
    (:3
      (Niagara|SpawnSystematLocation "/Game/TowerDefense/Stylized_VFX_StPack/Particles/UPDATE_1_2/P_Classic_Shot_03.P_Classic_Shot_03" _returnvalue_2 _returnvalue)))
  (CallFunction|Again))

(fn ConstructionScript)