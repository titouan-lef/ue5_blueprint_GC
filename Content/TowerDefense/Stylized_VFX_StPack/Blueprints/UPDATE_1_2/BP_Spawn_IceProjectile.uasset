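; Spawner Blueprint from a stylized VFX pack that repeatedly fires BP_Ice_Projectile from its own transform.
; BeginPlay waits a delay scaled by Level, which staggers spawners of different levels, then spawns the first projectile.
; Each spawn passes Gravity, ImpulsePower and Level to the projectile, then re-calls the Again event, which loops forever on a fixed delay.
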(event Custom|Again
  (Utilities|FlowControl|Delay 6.0)
  (Game|SpawnActorfromClass "/Game/TowerDefense/Stylized_VFX_StPack/Blueprints/UPDATE_1_2/BP_Ice_Projectile.BP_Ice_Projectile_C" (Transformation|GetActorTransform) "Undefined" "OverrideRootScale" 0 (Variables|Default|GetGravity) (Variables|Default|GetImpulse%20Power) (Variables|Default|GetLevel) 0)
  (CallFunction|Again))

(event EventBeginPlay
  (Utilities|FlowControl|Delay (* (Variables|Default|GetLevel) 2.0))
  (Game|SpawnActorfromClass "/Game/TowerDefense/Stylized_VFX_StPack/Blueprints/UPDATE_1_2/BP_Ice_Projectile.BP_Ice_Projectile_C" (Transformation|GetActorTransform) "Undefined" "OverrideRootScale" 0 (Variables|Default|GetGravity) (Variables|Default|GetImpulse%20Power) (Variables|Default|GetLevel) 0)
  (CallFunction|Again))

(fn ConstructionScript)