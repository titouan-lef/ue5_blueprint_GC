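; Life system that tracks current and maximum health and a death flag, with current health starting at maximum on BeginPlay.
; TakeDamage flags death only when health drops below zero, while Heal caps at maximum.
; Max health changes refuse negative results but never clamp current health.
; IncreaseMaxHealth compares current to the already raised maximum, so full health does not follow a positive increase.
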(event EventBeginPlay
  (Variables|Default|SetCurrentHealth (Variables|Default|GetMaxHealth)))

(fn TakeDamage
  (params (Amount :type Float%20%28double-precision%29))
  (Variables|Default|SetCurrentHealth (- (Variables|Default|GetCurrentHealth) Amount))
  (if (< (Variables|Default|GetCurrentHealth) 0.0)
    (Variables|Default|SetIsDead true)
    (else
      (Variables|Default|SetIsDead false))))

(fn Heal
  (params (Amount :type Float%20%28double-precision%29))
  (bind _maxhealth (Variables|Default|GetMaxHealth))
  (if (< (+ (Variables|Default|GetCurrentHealth) Amount) _maxhealth)
    (Variables|Default|SetCurrentHealth (+ (Variables|Default|GetCurrentHealth) Amount))
    (else
      (Variables|Default|SetCurrentHealth _maxhealth))))

(fn IncreaseMaxHealth
  (params (Amount :type Float%20%28double-precision%29))
  (Variables|Default|SetMaxHealth (+ Amount (Variables|Default|GetMaxHealth)))
  (if (== (Variables|Default|GetCurrentHealth) (Variables|Default|GetMaxHealth))
    (Variables|Default|SetCurrentHealth (Variables|Default|GetMaxHealth))))

(fn DecreaseMaxHealth
  (params (Amount :type Float%20%28double-precision%29))
  (if (< (- (Variables|Default|GetMaxHealth) Amount) 0.0)
    (Development|PrintString "Can't reduce more max health !")
    (else
      (Variables|Default|SetMaxHealth (- (Variables|Default|GetMaxHealth) Amount)))))

(fn IsDead?
  (return (Variables|Default|GetIsDead)))